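; Base actor for time-pausable objects: it eases a movement speed down to zero, holds it, then restores it.
; PauseObject derives a step interval and size from the slowdown time and iteration count, then starts a looping timer that lowers CurrentMovementSpeed.
; At zero it waits PauseTime, then a second timer ramps back to the default and clears IsPaused.
; The file only updates the speed value, printing debug messages, and moves nothing itself.
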(event `self.PauseObject`
  (params (PauseTime :type "Float (single-precision)") (SlowdownTime :type "Float (single-precision)"))
  (`self.CalculateNumberOfSteps` SlowdownTime)
  (if (not (`self.IsPaused`))
    (set `self.IsPaused` true)
    (`KismetSystemLibrary.PrintString` "Object Paused")
    (`KismetSystemLibrary.K2_SetTimerDelegate` (delegate `PauseIterration`) (`self.DeltaTimeAcceleration`) true)))

(event `PauseIterration`
  (if (<= (`self.CurrentMovementSpeed`) 0.0)
    (`KismetSystemLibrary.K2_PauseTimer` null "PauseIterration")
    (set `self.CurrentMovementSpeed` 0.0)
    (`KismetSystemLibrary.PrintString` "Full Pause" true true (struct :`R` 1.0 :`B` 0.835607 :`A` 1.0) 6.0)
    (`KismetSystemLibrary.Delay` (stale `self.PauseObject` PauseTime))
    (`self.UnpauseObjectEvent`)
    (`KismetSystemLibrary.K2_ClearTimer` null "PauseIterration")
    (else
      (bind _output_get (set `self.CurrentMovementSpeed` (- (`self.CurrentMovementSpeed`) (`self.DeltaSpeed`))))
      (`KismetSystemLibrary.PrintString` (`KismetStringLibrary.Conv_DoubleToString` _output_get)))))

(event `UnpauseObjectEvent`
  (`KismetSystemLibrary.K2_SetTimerDelegate` (delegate `UnpauseIterration`) (`self.DeltaTimeAcceleration`) true))

(event `UnpauseIterration`
  (if (>= (`self.CurrentMovementSpeed`) (`self.DefaultMovementSpeed`))
    (`KismetSystemLibrary.K2_PauseTimer` null "UnpauseIterration")
    (set `self.CurrentMovementSpeed` (`self.DefaultMovementSpeed`))
    (`KismetSystemLibrary.PrintString` "Full Unpause" true true (struct :`G` 1.0 :`B` 0.046783 :`A` 1.0) 6.0)
    (set `self.IsPaused` false)
    (`KismetSystemLibrary.K2_ClearTimer` null "UnpauseIterration")
    (else
      (bind _output_get (set `self.CurrentMovementSpeed` (+ (`self.CurrentMovementSpeed`) (`self.DeltaSpeed`))))
      (`KismetSystemLibrary.PrintString` (`KismetStringLibrary.Conv_DoubleToString` _output_get)))))

(fn `CalculateNumberOfSteps`
  (params (SlowDownTime :type "Float (double-precision)"))
  (set `self.DeltaTimeAcceleration` (/ SlowDownTime (`self.NumberOfIterations`)))
  (set `self.DeltaSpeed` (/ (`self.DefaultMovementSpeed`) (`self.NumberOfIterations`))))

(fn `UserConstructionScript`)